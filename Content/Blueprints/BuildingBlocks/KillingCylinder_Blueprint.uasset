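; KillingCylinder is a building-block actor that kills a player it hits once it has moved from its starting position.
; It records its location at BeginPlay, and on mesh hit requires the signed sum of its X, Y and Z offsets to exceed one unit either way.
; A qualifying hit on a HexPlayerCharacter calls KillPlayer on the HexArenaShooter game mode, crediting the victim's last attacker.
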(event OnComponentHit(StaticMeshComponent)
  (params (HitComponent :type Primitive%20Component%20Object%20Reference) (OtherActor :type Actor%20Object%20Reference) (OtherComp :type Primitive%20Component%20Object%20Reference) (NormalImpulse :type Vector :default "0, 0, 0") (Hit :type Hit%20Result%20Structure%20%28by%20ref%29))
  (bind _returnvalue (Transformation|GetActorLocation))
  (bind _startpos (Variables|Default|GetStartPos))
  (bind _returnvalue_2 (- _returnvalue _startpos))
  (bind _returnvalue_3 (+ (.x _returnvalue_2) (.y _returnvalue_2) (.z _returnvalue_2)))
  (if (or (> _returnvalue_3 1.0) (< _returnvalue_3 -1.0))
    (bind _ashex_player_character_bp (Utilities|Casting|CastToHexPlayerCharacter_BP OtherActor))
    (Default|KillPlayer (.AsHex%20Arena%20Shooter (Utilities|Casting|CastToHexArenaShooter (Game|GetGameMode))) (.AsHex%20Player%20Controller%20BP (Utilities|Casting|CastToHexPlayerController_BP (Pawn|GetController _ashex_player_character_bp))) (Variables|/Game/Blueprints/HexPlayerCharacter_BP.HexPlayerCharacter_BP_C|GetLastHitByID _ashex_player_character_bp))))

(event EventBeginPlay
  (Variables|Default|SetStartPos (Transformation|GetActorLocation)))

(fn ConstructionScript)