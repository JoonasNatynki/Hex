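; Lava hazard actor for the hex arena shooter that rises steadily and kills players it hits.
; Tick moves it up by RiseSpeed each frame, without sweep or delta-time scaling, so climb speed depends on frame rate.
; On Hit with a HexPlayerCharacter_BP, it calls KillPlayer on the HexArenaShooter game mode, passing the victim's controller and crediting LastHitByID as the killer.
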(event EventBeginPlay)

(event Collision|EventActorBeginOverlap
  (params (OtherActor :type Actor%20Object%20Reference)))

(event Collision|EventHit
  (params (MyComp :type Primitive%20Component%20Object%20Reference) (Other :type Actor%20Object%20Reference) (OtherComp :type Primitive%20Component%20Object%20Reference) (bSelfMoved :type Boolean) (HitLocation :type Vector :default "0, 0, 0") (HitNormal :type Vector :default "0, 0, 0") (NormalImpulse :type Vector :default "0, 0, 0") (Hit :type Hit%20Result%20Structure%20%28by%20ref%29))
  (bind _ashex_player_character_bp (Utilities|Casting|CastToHexPlayerCharacter_BP Other))
  (Default|KillPlayer (.AsHex%20Arena%20Shooter (Utilities|Casting|CastToHexArenaShooter (Game|GetGameMode))) (.AsHex%20Player%20Controller%20BP (Utilities|Casting|CastToHexPlayerController_BP (Pawn|GetController _ashex_player_character_bp))) (Variables|/Game/Blueprints/HexPlayerCharacter_BP.HexPlayerCharacter_BP_C|GetLastHitByID _ashex_player_character_bp)))

(event EventTick
  (params (DeltaSeconds :type Float%20%28single-precision%29))
  (Transformation|SetActorLocation (+ (Transformation|GetActorLocation) (Math|Vector|MakeVector 0.0 0.0 (Variables|Default|GetRiseSpeed))) false false))

(fn ConstructionScript)