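; Guillotine-style building block that moves a referenced static mesh actor when Execute fires, optionally at BeginPlay.
; Execute either enables physics on the mesh, optionally restoring its start position after a delay, or moves it toward a manual end position.
; A looping per-frame timer drives VInterpTo motion in both directions instead of Tick.
; Returns use interpolation or teleport, and completing the interpolated cycle clears Triggered to allow re-firing.
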(event Custom|Execute
  (if (not (Variables|Default|Gettriggered))
    (Variables|Default|Settriggered true)
    (if (Variables|Default|GetPhysics_On_When_Triggered_NoEndPos)
      (Physics|SetSimulatePhysics (Variables|/Script/Engine.StaticMeshActor|GetStaticMeshComponent (Variables|Default|GetActorReferenceForMeshComponent)) true)
      (if (Variables|Default|GetReturn_To_Start_State)
        (Utilities|FlowControl|Delay (Variables|Default|GetTime_Till_Return))
        (Physics|SetSimulatePhysics (Variables|/Script/Engine.StaticMeshActor|GetStaticMeshComponent (Variables|Default|GetActorReferenceForMeshComponent)) false)
        (if (Variables|Default|GetReturn_To_Start_State_Teleport)
          (Transformation|SetWorldLocation (Variables|/Script/Engine.StaticMeshActor|GetStaticMeshComponent (Variables|Default|GetActorReferenceForMeshComponent)) (Variables|Default|GetStartPos) false true)
          (else
            (Utilities|Time|SetTimerbyFunctionName 0 "VInterpToPos" (Utilities|Time|GetWorldDeltaSeconds) true))))
      (else
        (Utilities|Time|SetTimerbyFunctionName 0 "VInterpToPos" (Utilities|Time|GetWorldDeltaSeconds) true)))))

(event Custom|VInterpToPos
  (if (Variables|Default|GetTransform_To_EndPos_NOPHY)
    (Transformation|SetWorldLocation (Variables|/Script/Engine.StaticMeshActor|GetStaticMeshComponent (Variables|Default|GetActorReferenceForMeshComponent)) (Math|Interpolation|VInterpTo (Transformation|GetWorldLocation (Variables|/Script/Engine.StaticMeshActor|GetStaticMeshComponent (Variables|Default|GetActorReferenceForMeshComponent))) (Variables|Default|GetEndPos_For_Manual_Transform) (Utilities|Time|GetWorldDeltaSeconds) (Variables|Default|GetReturn_Speed)) false false)
    (if (Math|Vector|Equal(Vector) (Transformation|GetWorldLocation (Variables|/Script/Engine.StaticMeshActor|GetStaticMeshComponent (Variables|Default|GetActorReferenceForMeshComponent))) (Variables|Default|GetEndPos_For_Manual_Transform) 0.01)
      (if (Variables|Default|GetReturn_To_Start_State_VInterp)
        (Variables|Default|SetTransform_To_EndPos_NOPHY false)
        (elif true
          (Utilities|Time|ClearTimerbyFunctionName 0 "VInterpToPos")
          (Transformation|SetWorldLocation (Variables|/Script/Engine.StaticMeshActor|GetStaticMeshComponent (Variables|Default|GetActorReferenceForMeshComponent)) (Variables|Default|GetStartPos) false true)
          (Variables|Default|Settriggered false))))
    (else
      (Transformation|SetWorldLocation (Variables|/Script/Engine.StaticMeshActor|GetStaticMeshComponent (Variables|Default|GetActorReferenceForMeshComponent)) (Math|Interpolation|VInterpTo (Transformation|GetWorldLocation (Variables|/Script/Engine.StaticMeshActor|GetStaticMeshComponent (Variables|Default|GetActorReferenceForMeshComponent))) (Variables|Default|GetStartPos) (Utilities|Time|GetWorldDeltaSeconds) (Variables|Default|GetReturn_Speed)) false false)
      (if (Math|Vector|Equal(Vector) (Transformation|GetWorldLocation (Variables|/Script/Engine.StaticMeshActor|GetStaticMeshComponent (Variables|Default|GetActorReferenceForMeshComponent))) (Variables|Default|GetStartPos) 0.01)
        (Utilities|Time|ClearTimerbyFunctionName 0 "VInterpToPos")
        (Variables|Default|Settriggered false)))))

(event EventBeginPlay
  (Variables|Default|SetStartPos (Transformation|GetActorLocation (Variables|Default|GetActorReferenceForMeshComponent)))
  (Variables|Default|SetReturn_To_Start_State (or (Variables|Default|GetReturn_To_Start_State_Teleport) (Variables|Default|GetReturn_To_Start_State_VInterp)))
  (if (Variables|Default|GetExecuteOnBeginPlay)
    (Utilities|Time|SetTimerbyFunctionName 0 "Execute" (Utilities|Time|GetWorldDeltaSeconds))))

(fn ConstructionScript)