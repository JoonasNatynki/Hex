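; Short-lived explosion actor that pushes nearby objects and records which player caused the blast.
; On BeginPlay it fires its RadialForce impulse, then destroys itself after a brief delay.
; Characters overlapping its Sphere, other than the instigator, get their last-hit-by set to the PlayerID from the instigator controller's player settings.
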(event OnComponentBeginOverlap(Sphere)
  (params (OverlappedComponent :type Primitive%20Component%20Object%20Reference) (OtherActor :type Actor%20Object%20Reference) (OtherComp :type Primitive%20Component%20Object%20Reference) (OtherBodyIndex :type Integer) (bFromSweep :type Boolean) (SweepResult :type Hit%20Result%20Structure%20%28by%20ref%29))
  (bind _ashex_player_character_bp (Utilities|Casting|CastToHexPlayerCharacter_BP OtherActor))
  ;[1 1 1] Whoever gets affected by this explosion also gets LastHitByID in Character Blueprint set to this explosions instigators id
  (if (not (== (.AsHex%20Player%20Character%20BP (Utilities|Casting|CastToHexPlayerCharacter_BP (Game|GetInstigator))) _ashex_player_character_bp))
    (Default|SetLastHitby _ashex_player_character_bp (.PlayerID (Utilities|Struct|BreakPlayerInfo2 (Variables|/Game/Blueprints/HexPlayerController_BP.HexPlayerController_BP_C|GetPlayerSettings2 (.AsHex%20Player%20Controller%20BP (Utilities|Casting|CastToHexPlayerController_BP (Game|GetInstigatorController)))))))))

(event EventBeginPlay
  (Class|RadialForceComponent|FireImpulse (Variables|Default|GetRadialForce))
  (Utilities|FlowControl|Delay 4.0)
  (Actor|DestroyActor))

(event Collision|EventActorBeginOverlap
  (params (OtherActor :type Actor%20Object%20Reference)))

(event EventTick
  (params (DeltaSeconds :type Float%20%28single-precision%29)))

(fn ConstructionScript)