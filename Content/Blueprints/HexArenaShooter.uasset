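; Game mode for the Hex Arena shooter that tracks connected player controllers and runs the round countdown.
; BeginPlay loads the round time from GameInfoInstance and starts a server-side one-second timer that decrements it, clearing RoundOn at zero.
; Swapped-in controllers receive the current time once, and logout asks the game instance to destroy that player's session.
; The construction script sets console variables for long-distance dynamic shadows.
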(event Custom|StartRoundTimer
  ;[1 1 1] Round time
  (Utilities|Time|SetTimerbyEvent (delegate Custom|UpdateRoundTime) 1.0 (Variables|RoundTime|GetRoundOn)))

(event Custom|UpdateRoundTime
  ;[1 1 1] Round time
  (if (< (Variables|RoundTime|GetCurrentRoundTime) 1)
    (Variables|RoundTime|SetRoundOn false)
    (else
      (Variables|RoundTime|SetCurrentRoundTime (- (Variables|RoundTime|GetCurrentRoundTime) 1)))))

(event EventBeginPlay
  (bind _returnvalue (Game|GetGameInstance))
  (bind _asgame_info_instance (Utilities|Casting|CastToGameInfoInstance _returnvalue))
  (Variables|Default|SetGameInstanceRef _asgame_info_instance)
  (Variables|RoundTime|SetCurrentRoundTime (Variables|/Game/Blueprints/GameInfoInstance.GameInfoInstance_C|GetRoundTime _asgame_info_instance))
  (if (Networking|IsServer)
    (CallFunction|StartRoundTimer)))

(event EventTick
  (params (DeltaSeconds :type Float%20%28single-precision%29)))

(event EventOnSwapPlayerControllers
  (params (OldPC :type Player%20Controller%20Object%20Reference) (NewPC :type Player%20Controller%20Object%20Reference))
  ;[1 1 1] Keeps track of connected player controllers and give controller info about round time
  (bind _ashex_player_controller_bp (Utilities|Casting|CastToHexPlayerController_BP NewPC))
  (Utilities|Array|Add (Variables|Default|GetAllPlayerControllers) _ashex_player_controller_bp)
  (Default|UpdateRoundTime _ashex_player_controller_bp (Variables|RoundTime|GetCurrentRoundTime)))

(event EventOnLogout
  (params (ExitingController :type Controller%20Object%20Reference))
  ;[1 1 1] OnLogout destroy session
  (bind _ashex_player_controller_bp (Utilities|Casting|CastToHexPlayerController_BP ExitingController))
  (Default|DestroySessionCaller (Variables|Default|GetGameInstanceRef) _ashex_player_controller_bp))

(fn ConstructionScript
  ;[1 1 1] Dynamic shadows draw very far away and quite well
  (Development|ExecuteConsoleCommand "r.Shadow.FadeResolution 12")
  (Development|ExecuteConsoleCommand "r.Shadow.MinResolution 1")
  (Development|ExecuteConsoleCommand "r.Shadow.TexelsPerPixel 0.01")
  (Development|ExecuteConsoleCommand "r.Shadow.RadiusThreshold 0.001"))

(fn OnRepRoundon)