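; Player character with a socket-mounted camera, camera-relative movement, walk/run toggle and free look, spawning with an equipped weapon.
; Tick traces from the camera for an aim point, derives clamped torso pitch/yaw, turns the body past a yaw threshold, and freezes movement during round freeze.
; Held fire repeatedly messages the weapon through an interface.
; Sprint speed and recovery logic exists, but sprint toggles and physical animation are unwired.
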(event EventBeginPlay
  ;[1 1 1] Dynamic shadows draw very far away and quite well
  (Development|ExecuteConsoleCommand "r.Shadow.FadeResolution 12")
  (Development|ExecuteConsoleCommand "r.Shadow.MinResolution 2")
  (Development|ExecuteConsoleCommand "r.Shadow.TexelsPerPixel 0.01")
  (Development|ExecuteConsoleCommand "r.Shadow.RadiusThreshold 0.001")
  (bind _returnvalue (Game|SpawnActorfromClass "/Game/Blueprints/Weapon_Item_BP.Weapon_Item_BP_C" (Transformation|GetActorTransform) "AlwaysSpawn" 0 0))
  (Variables|Default|SetEquippedItem _returnvalue)
  (CallFunction|WeaponPickUp _returnvalue))

(event Collision|EventActorBeginOverlap
  (params (OtherActor :type Actor%20Object%20Reference)))

(event EventPickupNotify
  (params (item :type Actor%20Object%20Reference))
  (bind _asweapon_item_bp (Utilities|Casting|CastToWeapon_Item_BP item)) ; If weapon
  (CallFunction|WeaponPickUp _asweapon_item_bp))

(event EventTick
  (params (DeltaSeconds :type Float%20%28single-precision%29))
  (bind _returnvalue (Pawn|GetControlRotation :!class /Script/Engine.Pawn))
  (bind _returnvalue_2 (Transformation|GetActorRotation))
  (bind _returnvalue_3 (Pawn|GetControlRotation :!class /Script/Engine.Pawn))
  (bind _charactermovement (Variables|Character|GetCharacterMovement))
  (bind _aimretargetspeed (Variables|Default|GetAimRetargetSpeed))
  (bind _camera (Variables|Default|GetCamera))
  (bind _charactermovement_2 (Variables|Character|GetCharacterMovement))
  (bind _torsomaxrotation (Variables|Default|GetTorsoMaxRotation))
  (bind _charactermovement_3 (Variables|Character|GetCharacterMovement))
  (bind _returnvalue_4 (Transformation|GetWorldLocation _camera))
  (bind _returnvalue_5 (Math|Rotator|Delta(Rotator) _returnvalue _returnvalue_2))
  (bind _pitch (Math|Rotator|BreakRotator _returnvalue_3))
  (bind _yaw (Math|Rotator|BreakRotator _returnvalue_5))
  ;[1 1 1] If round state is "NewRoundFreeze" then disable movement
  (if (Utilities|Enum|Equal(Enum) (Variables|/Game/Blueprints/HexPlayerController_BP.HexPlayerController_BP_C|GetRoundState (.AsHex%20Player%20Controller%20BP (Utilities|Casting|CastToHexPlayerController_BP (Game|GetPlayerController 0)))) "NewEnumerator3")
    (Pawn|Components|CharacterMovement|SetMovementMode _charactermovement_2 "MOVE_None" 0)
    (elif (Utilities|Enum|Equal(Enum) (Variables|/Script/Engine.CharacterMovementComponent|GetMovementMode (Variables|Character|GetCharacterMovement)) "MOVE_None")
      (Pawn|Components|CharacterMovement|SetMovementMode _charactermovement_2 "MOVE_Walking" 0)))
  (Utilities|FlowControl|Sequence
    (:then_0
      ;[1 1 1] Do a traceline to where the player is aiming at
      (if true
        (bind (_outhit _returnvalue_6) (Collision|LineTraceByChannel _returnvalue_4 (+ (* (Math|Vector|GetForwardVector _camera) 1e+03) _returnvalue_4) "TraceTypeQuery2" false 0 "None" true "(R=1.000000,G=0.000000,B=0.000000,A=1.000000)" "(R=0.000000,G=1.000000,B=0.000000,A=1.000000)" 1.0))
        (Variables|Default|SetTimeSinceLastAimRetarget 0.0)
        (else
          (Variables|Default|SetTimeSinceLastAimRetarget (+ (Variables|Default|GetTimeSinceLastAimRetarget) DeltaSeconds)))))
    (:then_1
      (if _returnvalue_6
        (Variables|Default|SetAimingPosition (.ImpactPoint (Collision|BreakHitResult _outhit)))
        (else
          (Variables|Default|SetAimingPosition (Math|Vector|MakeVector (Math|Interpolation|FInterpTo (.X (Math|Vector|BreakVector (Variables|Default|GetAimingPosition))) (.X (Math|Vector|BreakVector (.TraceEnd (Collision|BreakHitResult _outhit)))) DeltaSeconds _aimretargetspeed) (Math|Interpolation|FInterpTo (.Y (Math|Vector|BreakVector (Variables|Default|GetAimingPosition))) (.Y (Math|Vector|BreakVector (.TraceEnd (Collision|BreakHitResult _outhit)))) DeltaSeconds _aimretargetspeed) (Math|Interpolation|FInterpTo (.Z (Math|Vector|BreakVector (Variables|Default|GetAimingPosition))) (.Z (Math|Vector|BreakVector (.TraceEnd (Collision|BreakHitResult _outhit)))) DeltaSeconds _aimretargetspeed)))))
      ;[1 1 1] Handle aiming pitch
      ;;[1 1 1] Skip if FreeLook is on
      (if (Variables|Default|GetIsFreeLookOn)
        _
        (else
          (if (> _pitch 9e+01)
            (Variables|Default|SetPitch (- _pitch 3.6e+02))
            (else
              (Variables|Default|SetPitch _pitch)))
          ;[1 1 1] Handle aiming yaw, clamp values
          ;;[1 1 1] Skip if FreeLook is on
          (if (Variables|Default|GetIsFreeLookOn)
            _
            (elif (> _yaw (Variables|Default|GetAngleToStartRotatingHips))
              (Variables|Default|SetYaw (Math|Float|ClampAngle (- _yaw 3.6e+02) (* -1 _torsomaxrotation) _torsomaxrotation))
              (else
                (Variables|Default|SetYaw (Math|Float|ClampAngle _yaw (* -1 _torsomaxrotation) _torsomaxrotation)))))))
      (Utilities|FlowControl|Sequence
        (:then_0
          ;[1 1 1] Spool max running speed when sprinting
          (if (Variables|Default|GetIsSprinting)
            (Variables|/Script/Engine.CharacterMovementComponent|SetMaxWalkSpeed _charactermovement_3 (Math|Interpolation|FInterpTo (Math|Vector|VectorLength (Variables|/Script/Engine.MovementComponent|GetVelocity _charactermovement_3)) (Variables|Default|GetSprintSpeed) DeltaSeconds 5.0))
            (elif (Variables|Default|GetIsRunning)
              (Variables|/Script/Engine.CharacterMovementComponent|SetMaxWalkSpeed _charactermovement_3 (Variables|Default|GetRunSpeed))
              (else
                (Variables|/Script/Engine.CharacterMovementComponent|SetMaxWalkSpeed _charactermovement_3 (Variables|Default|GetWalkSpeed))))))
        (:then_1
          ;[1 1 1] Turn hips if the aim turns too much
          (if (Variables|Default|GetHasEquippedItemReady)
            (Variables|Default|SetAngleToStartRotatingHips (Variables|Default|GetAngleToStartRotatingHips))
            (else
              (Variables|Default|SetAngleToStartRotatingHips (Variables|Default|GetAngleToStartRotatingHipsWide))))
          (if (> (Math|Float|Absolute(Float) (Variables|Default|GetYaw)) (Variables|Default|GetAngleToStartRotatingHips))
            (Transformation|SetActorRotation (Math|Interpolation|RInterpTo (Math|Rotator|MakeRotator 0.0 0.0 (.Yaw (Math|Rotator|BreakRotator (Transformation|GetActorRotation)))) (Math|Rotator|MakeRotator 0.0 0.0 (.Yaw (Math|Rotator|BreakRotator (Pawn|GetControlRotation :!class /Script/Engine.Pawn)))) DeltaSeconds 2.0))))
        (:then_2
          ;[1 1 1] Recovery from sprinting
          (if (> (Math|Vector|VectorLength (Variables|/Script/Engine.MovementComponent|GetVelocity _charactermovement)) (+ (Variables|Default|GetRunSpeed) 2e+01))
            (Variables|/Script/Engine.CharacterMovementComponent|SetMaxAcceleration _charactermovement (Variables|Default|GetDefaultSprintingAcceleration))
            (Variables|/Script/Engine.CharacterMovementComponent|SetBrakingDecelerationWalking _charactermovement 3e+02)
            (else
              (Variables|/Script/Engine.CharacterMovementComponent|SetMaxAcceleration _charactermovement (Math|Interpolation|FInterptoConstant (Class|CharacterMovementComponent|GetMaxAcceleration _charactermovement) (Variables|Default|GetDefaultRunningAcceleration2) DeltaSeconds (Variables|Default|GetSprintingAccelerationRecoveryInterpSpeed)))
              (Variables|/Script/Engine.CharacterMovementComponent|SetBrakingDecelerationWalking _charactermovement (Variables|Default|GetDefaultBreakingAcceleration)))))))))

(event Input|ActionEvents|InputActionFire
  (params (Key :type Key%20Structure :default "AnyKey"))
  (bind _equippeditem (Variables|Default|GetEquippedItem))
  (:Pressed
    (Variables|Default|SetIsFiring true)
    (if (Variables|Default|GetIsFiring) :!label _label
      (if (Utilities|DoesObjectImplementInterface _equippeditem "/Game/Blueprints/Weapon_Interface.Weapon_Interface_C")
        (Class|WeaponInterface|Fire(Message) _equippeditem)
        (Utilities|FlowControl|Delay 1.0)
        (goto _label))))
  (:Released
    (Variables|Default|SetIsFiring false)))

(event Input|ActionEvents|InputActionFreeLook
  (params (Key :type Key%20Structure :default "AnyKey"))
  ;[1 1 1] FreeLook
  (:Pressed
    (if (Variables|Default|GetIsFreeLookOn)
      (Variables|Default|SetIsFreeLookOn false)
      (else
        (Variables|Default|SetIsFreeLookOn true)))))

(event Input|ActionEvents|InputActionSprint
  (params (Key :type Key%20Structure :default "AnyKey"))
  ;[1 1 1] Walking/Running/Sprinting
)

(event Input|ActionEvents|InputActionWalk/Run
  (params (Key :type Key%20Structure :default "AnyKey"))
  (bind _charactermovement (Variables|Character|GetCharacterMovement))
  ;[1 1 1] Walking/Running/Sprinting
  (:Pressed
    (if (Variables|Default|GetIsRunning)
      (Variables|Default|SetIsRunning false)
      (Variables|/Script/Engine.CharacterMovementComponent|SetMaxWalkSpeed _charactermovement (Variables|Default|GetWalkSpeed))
      (else
        (Variables|Default|SetIsRunning true)
        (Variables|/Script/Engine.CharacterMovementComponent|SetMaxWalkSpeed _charactermovement (Variables|Default|GetRunSpeed))))))

(event Input|AxisEvents|InputAxisMoveForward
  (params (AxisValue :type Float%20%28single-precision%29))
  ;[1 1 1] When moving, orient character forward(camera view)
  (if (!= AxisValue 0.0)
    (Transformation|SetActorRotation (Math|Interpolation|RInterpTo (Math|Rotator|MakeRotator 0.0 0.0 (.Yaw (Math|Rotator|BreakRotator (Transformation|GetActorRotation)))) (Math|Rotator|MakeRotator 0.0 0.0 (.Yaw (Math|Rotator|BreakRotator (Pawn|GetControlRotation :!class /Script/Engine.Pawn)))) (stale EventTick DeltaSeconds) 5.0))
    (Pawn|Input|AddMovementInput (Math|Vector|RotateVectorAroundAxis (Transformation|GetActorRightVector (Pawn|GetController)) -9e+01 "0, 0,1.000000") AxisValue false)))

(event Input|AxisEvents|InputAxisMoveRight3
  (params (AxisValue :type Float%20%28single-precision%29))
  ;[1 1 1] When moving, orient character forward(camera view)
  (if (!= AxisValue 0.0)
    (Transformation|SetActorRotation (Math|Interpolation|RInterpTo (Math|Rotator|MakeRotator 0.0 0.0 (.Yaw (Math|Rotator|BreakRotator (Transformation|GetActorRotation)))) (Math|Rotator|MakeRotator 0.0 0.0 (.Yaw (Math|Rotator|BreakRotator (Pawn|GetControlRotation :!class /Script/Engine.Pawn)))) (stale EventTick DeltaSeconds) 5.0))
    (Pawn|Input|AddMovementInput (Transformation|GetActorRightVector (Pawn|GetController)) AxisValue false)))

(fn ConstructionScript
  (bind _camera (Variables|Default|GetCamera))
  (bind _charactermovement (Variables|Character|GetCharacterMovement))
  (bind _returnvalue (Math|Vector|GetForwardVector _camera))
  (bind _returnvalue_2 (Transformation|GetWorldLocation _camera))
  (bind _returnvalue_3 (* _returnvalue 1e+03))
  (bind _returnvalue_4 (+ _returnvalue_3 _returnvalue_2))
  (Transformation|AttachComponentToComponent (Variables|Default|GetCamera) (Variables|Character|GetMesh) "camera_socket" "SnapToTarget" "KeepRelative" "KeepRelative" true)
  (Collision|LineTraceByChannel _returnvalue_2 _returnvalue_4 "TraceTypeQuery2" false 0 "None")
  (Variables|Default|SetAimingPosition _returnvalue_4)
  (Variables|/Script/Engine.CharacterMovementComponent|SetMaxWalkSpeed _charactermovement (Variables|Default|GetRunSpeed))
  (Variables|/Script/Engine.CharacterMovementComponent|SetGroundFriction _charactermovement (Variables|Default|GetDefaultGroundFriction))
  (Variables|/Script/Engine.CharacterMovementComponent|SetMaxAcceleration _charactermovement (Variables|Default|GetDefaultRunningAcceleration2))
  (Variables|/Script/Engine.CharacterMovementComponent|SetBrakingDecelerationWalking _charactermovement (Variables|Default|GetDefaultBreakingAcceleration))
  (Variables|/Script/Engine.CharacterMovementComponent|SetBrakingFriction _charactermovement 11.0)
  ;[1 1 1] Dynamic shadows draw very far away and quite well
  (Development|ExecuteConsoleCommand "r.Shadow.FadeResolution 12")
  (Development|ExecuteConsoleCommand "r.Shadow.MinResolution 2")
  (Development|ExecuteConsoleCommand "r.Shadow.TexelsPerPixel 0.01")
  (Development|ExecuteConsoleCommand "r.Shadow.RadiusThreshold 0.001"))

(fn WeaponPickUp
  (params (Weapon :type Item%20Object%20Reference))
  (bind _mesh (Variables|/Script/Hex.Item|Getmesh Weapon))
  (Physics|SetSimulatePhysics _mesh false)
  (Collision|SetCollisionResponsetoChannel _mesh "ECC_Pawn" "ECR_Ignore")
  (Collision|SetCollisionResponsetoChannel _mesh "ECC_Camera" "ECR_Ignore")
  (Variables|Default|SetEquippedItem Weapon)
  (Variables|/Script/Hex.Item|SetIsPickedUp Weapon true)
  (Transformation|AttachComponentToComponent _mesh (Variables|Character|GetMesh) "weapon_socket" "SnapToTarget" "SnapToTarget" "KeepRelative" true)
  (Transformation|AddLocalOffset (Variables|/Script/Hex.Item|Getmesh Weapon) (* (Math|Transform|InverseTransformLocation (Transformation|GetWorldTransform _mesh) (Transformation|GetSocketLocation _mesh "RightHandHold")) -1) false false) ; lefhandhold offset
  (bind _asweapon_item_bp (Utilities|Casting|CastToWeapon_Item_BP Weapon))
  (Variables|/Game/Blueprints/Weapon_Item_BP.Weapon_Item_BP_C|SetOwnedBy _asweapon_item_bp self))