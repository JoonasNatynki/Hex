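; Lobby GameMode that tracks joining players, map settings and team assignments, then launches the match.
; PostLogin registers each LobbyPC, gives it an incremental PlayerID, reads server info from GameInfoInstance and sends current settings.
; Setting changes push to every LobbyPC, while EveryoneUpdate rebuilds and redistributes the player list and count, including after team changes.
; LaunchTheGame seamlessly server-travels to the level matching the selected map ID.
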(event Custom|LaunchTheGame
  (bind _returnvalue (Game|GetPlayerController 0))
  ;[1 1 1] Launches the game
  (Variables|Default|SetbUseSeamlessTravel true)
  (switch int (Variables|ServerSettings|GetGM_MapID)
    (:0
      (Development|ExecuteConsoleCommand "servertravel /Game/TestLevel" _returnvalue))
    (:1
      (Development|ExecuteConsoleCommand "servertravel /Game/Maps/DRAFT" _returnvalue))))

(event Custom|EveryoneUpdate
  (bind _allplayercontrollers (Variables|ServerSettings|GetAllPlayerControllers))
  ;[1 1 1] EveryoneUpdate
  (bind _output_get (Variables|ServerSettings|SetCurrentPlayers (Utilities|Array|Length (Variables|ServerSettings|GetAllPlayerControllers))))
  (if (> _output_get 0)
    (Utilities|Array|Clear (Variables|Default|GetConnectedPlayers2))
    (for _array_element _allplayercontrollers
      (bind _aslobby_pc (Utilities|Casting|CastToLobbyPC _array_element))
      (Utilities|Array|Add (Variables|Default|GetConnectedPlayers2) (Variables|/Game/Blueprints/Lobby/LobbyPC.LobbyPC_C|GetPlayerSettings2 _aslobby_pc))
      (Default|UpdateNumberOfPlayers _aslobby_pc (Variables|ServerSettings|GetCurrentPlayers) (Variables|ServerSettings|GetMaxPlayers)))
    (for _array_element_2 _allplayercontrollers
      (bind _aslobby_pc_2 (Utilities|Casting|CastToLobbyPC _array_element_2))
      (Default|AddPlayerInfo _aslobby_pc_2 (Variables|Default|GetConnectedPlayers2)))))

(event Custom|AssignTeam
  (params (PlayersIndex :type Integer) (NewTeamIndex :type Integer))
  ;[1 1 1] Find the playercontroller whose team should change - Call Assign team function on that specific player controller
  (for _array_element (Variables|Default|GetConnectedPlayers2)
    (if (== (.PlayerID (Utilities|Struct|BreakPlayerInfo2 _array_element)) PlayersIndex)
      (bind _aslobby_pc (Utilities|Casting|CastToLobbyPC (Utilities|Array|Get(acopy) (Variables|ServerSettings|GetAllPlayerControllers) PlayersIndex)))
      (Default|AssignTeam _aslobby_pc NewTeamIndex)
      (CallFunction|EveryoneUpdate))))

(event Custom|ServerUpdateGameSettings
  (params (MapImage :type Texture%202D%20Object%20Reference) (MapName :type Text) (MapTime :type Text) (MapID :type Integer))
  ;[1 1 1] Server makes changes to game settings
  (Variables|ServerSettings|SetGM_MapImage MapImage)
  (Variables|ServerSettings|SetGM_MapName MapName)
  (Variables|ServerSettings|SetGM_MapTime MapTime)
  (Variables|ServerSettings|SetGM_MapID MapID)
  (for _array_element (Variables|ServerSettings|GetAllPlayerControllers)
    (bind _aslobby_pc (Utilities|Casting|CastToLobbyPC _array_element))
    (Default|UpdateLobbySettings _aslobby_pc (Variables|ServerSettings|GetGM_MapImage) (Variables|ServerSettings|GetGM_MapName) (Variables|ServerSettings|GetGM_MapTime))))

(event EventPostLogin
  (params (NewPlayer :type Player%20Controller%20Object%20Reference))
  ;[1 1 1] PostLogin
  (Networking|SwitchHasAuthority
    (:Authority
      (Utilities|Array|Add (Variables|ServerSettings|GetAllPlayerControllers) NewPlayer)
      (bind _outactors (Actor|GetAllActorsOfClass "/Script/Engine.PlayerStart"))
      (Variables|ServerSettings|SetSpawnPoints _outactors)
      (bind _asgame_info_instance (Utilities|Casting|CastToGameInfoInstance (Game|GetGameInstance)))
      (Variables|ServerSettings|SetServerName (Variables|/Game/Blueprints/GameInfoInstance.GameInfoInstance_C|GetServerName _asgame_info_instance))
      (Variables|ServerSettings|SetMaxPlayers (Variables|/Game/Blueprints/GameInfoInstance.GameInfoInstance_C|GetNumberOfPlayers _asgame_info_instance))
      (bind _aslobby_pc (Utilities|Casting|CastToLobbyPC NewPlayer))
      (Default|SetupLobbyMenu _aslobby_pc (Variables|ServerSettings|GetServerName))
      (Default|InitialSetup _aslobby_pc)
      (Utilities|Struct|SetmembersinPlayerInfo2 (Variables|/Game/Blueprints/Lobby/LobbyPC.LobbyPC_C|GetPlayerSettings2 _aslobby_pc) (Variables|Default|GetNextID))
      (Variables|Default|SetNextID (+ (Variables|Default|GetNextID) 1))
      (Default|Save _aslobby_pc)
      (Default|UpdateLobbySettings _aslobby_pc (Variables|ServerSettings|GetGM_MapImage) (Variables|ServerSettings|GetGM_MapName) (Variables|ServerSettings|GetGM_MapTime)))))

(fn ConstructionScript)