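; PlayerGibs is an actor that produces a gore burst, shattering a destructible player-character mesh and scattering gibs.
; On BeginPlay it applies heavy damage to the destructible mesh, with a randomized impulse along the actor's velocity.
; It then runs two self-feeding DoN loops with random limits, spawning Gib_1_persistent and Gib_1 actors at jittered offsets.
; Each gib's collision box gets a radial impulse from the actor's location.
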(event EventBeginPlay
  (bind _returnvalue (Math|Random|RandomIntegerinRange 20 50))
  (bind _returnvalue_2 (Transformation|GetActorLocation))
  (bind _returnvalue_3 (Math|Random|RandomFloatinRange -25.0 25.0))
  (bind _returnvalue_4 (Math|Random|RandomFloatinRange -25.0 25.0))
  (bind _returnvalue_5 (Math|Random|RandomFloatinRange -25.0 25.0))
  (bind _returnvalue_6 (Math|Vector|MakeVector _returnvalue_3 _returnvalue_4 _returnvalue_5))
  (bind _returnvalue_7 (+ _returnvalue_2 _returnvalue_6))
  (bind _returnvalue_8 (Math|Conversions|ToTransform(Vector) _returnvalue_7))
  (Game|Damage|ApplyDamage (Variables|Default|GetHexCharacterDestructibleMesh_DM) 1e+03 (+ (Transformation|GetActorLocation) (Math|Vector|MakeVector (Math|Random|RandomFloatinRange 2e+01 25.0) 0.0 (Math|Random|RandomFloatinRange 17.0 22.0))) (Transformation|GetVelocity) (Math|Random|RandomFloatinRange 7e+02 2.5e+03))
  (Utilities|FlowControl|Sequence
    (:then_0
      (bind _counter (Utilities|FlowControl|DoN _returnvalue :!label _label)
        (:Exit
          (if (>= (Math|Conversions|ToFloat(Integer) _counter) (Math|Conversions|ToFloat(Integer) _returnvalue))
            (goto _label Reset)
            (else
              (bind _returnvalue_9 (Game|SpawnActorfromClass "/Game/Blueprints/Gibs/Bug_1_Gibs/Gib_1_persistent.Gib_1_persistent_C" _returnvalue_8 "AdjustIfPossibleButAlwaysSpawn" 0 0))
              (Physics|AddRadialImpulse (Variables|/Game/Blueprints/Gibs/Bug_1_Gibs/Gib_1_persistent.Gib_1_persistent_C|GetCollision_Box _returnvalue_9) (Transformation|GetActorLocation) 1e+02 8e+03 "RIF_Constant" false)
              (goto _label))))))
    (:then_1
      (bind _returnvalue_10 (Game|SpawnActorfromClass "/Game/Blueprints/Gibs/Bug_1_Gibs/Gib_1.Gib_1_C" _returnvalue_8 "AdjustIfPossibleButAlwaysSpawn" 0 0 :!label _label_2)) ; permanent gibs
      (Physics|AddRadialImpulse (Variables|/Game/Blueprints/Gibs/Bug_1_Gibs/Gib_1.Gib_1_C|GetCollision_Box _returnvalue_10) (Transformation|GetActorLocation) 1e+02 8e+03 "RIF_Constant" false)
      (Utilities|FlowControl|DoN (Math|Random|RandomIntegerinRange 20 50)
        (:Exit
          (goto _label_2))))))

(event Collision|EventActorBeginOverlap
  (params (OtherActor :type Actor%20Object%20Reference)))

(event EventTick
  (params (DeltaSeconds :type Float%20%28single-precision%29)))

(fn ConstructionScript)