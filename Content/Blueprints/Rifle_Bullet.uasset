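; Rifle_Bullet is a projectile Blueprint that explodes when it hits something.
; On BeginPlay it sets up collision ignores for the owning HexPlayerCharacter_BP and its equipped item, and registers itself with that character to be ignored.
; On Hit it prints debug checks on distance from below the owner and the hit component, spawns a half-scale Explosion_1 at impact, plays Frag_explosion at world origin, then destroys itself.
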(event EventBeginPlay
  (bind _returnvalue (Components|GetOwner))
  (bind _collisioncomponent (Variables|Default|GetCollisionComponent))
  (bind _ashex_player_character_bp (Utilities|Casting|CastToHexPlayerCharacter_BP _returnvalue))
  (Collision|IgnoreActorwhenMoving _collisioncomponent _returnvalue true)
  (Collision|IgnoreActorwhenMoving _collisioncomponent (Variables|/Game/Blueprints/HexPlayerCharacter_BP.HexPlayerCharacter_BP_C|GetEquippedItem _ashex_player_character_bp) true)
  (Collision|IgnoreActorwhenMoving _collisioncomponent _ashex_player_character_bp true)
  (Default|SetActortoIgnore _ashex_player_character_bp self))

(event Collision|EventActorBeginOverlap
  (params (OtherActor :type Actor%20Object%20Reference)))

(event EventTick
  (params (DeltaSeconds :type Float%20%28single-precision%29)))

(event Collision|EventHit
  (params (MyComp :type Primitive%20Component%20Object%20Reference) (Other :type Actor%20Object%20Reference) (OtherComp :type Primitive%20Component%20Object%20Reference) (bSelfMoved :type Boolean) (HitLocation :type Vector) (HitNormal :type Vector :default "0, 0, 0") (NormalImpulse :type Vector :default "0, 0, 0") (Hit :type Hit%20Result%20Structure%20%28by%20ref%29))
  (bind _returnvalue (Components|GetOwner))
  (bind _returnvalue_2 (Transformation|GetActorTransform _returnvalue))
  (bind _location (Math|Transform|BreakTransform _returnvalue_2))
  (bind _returnvalue_3 (+ _location "0, 0,-97.000000"))
  (bind _returnvalue_4 (- HitLocation _returnvalue_3))
  (bind _returnvalue_5 (Math|Vector|VectorLength _returnvalue_4))
  (if (< _returnvalue_5 51.0)
    (Development|PrintString "true")
    (else
      (Development|PrintString (Utilities|String|ToString(Float) _returnvalue_5))))
  (Development|PrintString (Utilities|GetDisplayName OtherComp))
  (bind _returnvalue_6 (Game|SpawnActorfromClass "/Game/Blueprints/Explosion_1.Explosion_1_C" (Math|Conversions|ToTransform(Vector) (.ImpactPoint (Collision|BreakHitResult Hit))) "Undefined" 0 0))
  (Transformation|SetWorldScale3D (Variables|/Game/Blueprints/Explosion_1.Explosion_1_C|GetDefaultSceneRoot _returnvalue_6) "0.500000,0.500000,0.500000")
  (Audio|SpawnSoundatLocation "/Game/BallisticsVFX/SFX/Explodes/Wav/Frag_explosion.Frag_explosion" "0, 0, 0")
  (Actor|DestroyActor))

(fn ConstructionScript)