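; Weapon item actor, a rifle that a HexPlayerCharacter can pick up and fire.
; On BeginPlay it stores the left-hand grip offset from the right-hand socket in mesh space and prints it; a mesh hit by a HexPlayerCharacter sends that character a pickup notice.
; Fire spawns a bullet owned by the holder with sound, muzzle flash and camera shake, then kicks the holder's view with pitch and random yaw recoil.
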(event OnComponentHit(mesh)
  (params (HitComponent :type Primitive%20Component%20Object%20Reference) (OtherActor :type Actor%20Object%20Reference) (OtherComp :type Primitive%20Component%20Object%20Reference) (NormalImpulse :type Vector :default "0, 0, 0") (Hit :type Hit%20Result%20Structure%20%28by%20ref%29))
  (if (not false)
    (bind _ashex_player_character (Utilities|Casting|CastToHexPlayerCharacter OtherActor))
    (Class|HexPlayerCharacter|PickupNotify _ashex_player_character self)))

(event EventBeginPlay
  (bind _mesh (Variables|Character|GetMesh))
  (bind _returnvalue (Transformation|GetSocketLocation _mesh "LeftHandHold"))
  (bind _returnvalue_2 (Transformation|GetSocketLocation _mesh "RightHandHold"))
  (bind _returnvalue_3 (Transformation|GetWorldTransform _mesh))
  (bind _returnvalue_4 (Math|Transform|InverseTransformLocation _returnvalue_3 _returnvalue_2))
  (bind _returnvalue_5 (Math|Transform|InverseTransformLocation _returnvalue_3 _returnvalue))
  (bind _returnvalue_6 (- _returnvalue_5 _returnvalue_4))
  (Variables|Default|SetLeftHandOffset _returnvalue_6)
  (Development|PrintString (Utilities|String|ToString(Vector) _returnvalue_6)))

(event Collision|EventActorBeginOverlap
  (params (OtherActor :type Actor%20Object%20Reference)))

(event EventTick
  (params (DeltaSeconds :type Float%20%28single-precision%29)))

(event EventFireWeapon)

(fn ConstructionScript)

(fn Fire
  (params (FiringVector :type Transform))
  (bind (_location _rotation) (Math|Transform|BreakTransform FiringVector))
  (Game|SpawnActorfromClass "/Game/Blueprints/Rifle_Bullet.Rifle_Bullet_C" FiringVector "AlwaysSpawn" (Variables|Default|GetOwnedBy) 0)
  (Audio|SpawnSoundatLocation "/Game/BallisticsVFX/SFX/Guns/Wav/AssaultRifle_Suppressed_2.AssaultRifle_Suppressed_2" _location "0, 0, 0" 3.0 1.0 0.0 "/Game/BallisticsVFX/SFX/Attentuations/Gun_Attenuation.Gun_Attenuation")
  (Effects|SpawnEmitteratLocation "/Game/BallisticsVFX/Particles/Muzzle/MuzzleFlash/Muzzle_Flash_Large.Muzzle_Flash_Large" _location _rotation)
  (Camera|PlayWorldCameraShake "/Game/Blueprints/Rifle_Camera_Shake.Rifle_Camera_Shake_C" (Transformation|GetWorldLocation (Variables|Character|GetMesh self)) 0.0 5e+01 0.1)
  (bind _ashex_player_character_bp (Utilities|Casting|CastToHexPlayerCharacter_BP (Variables|Default|GetOwnedBy))
    (:then
      (Pawn|Input|AddControllerPitchInput _ashex_player_character_bp -0.5)
      (Pawn|Input|AddControllerYawInput _ashex_player_character_bp (Math|Random|RandomFloatinRange -0.5 0.5)))
    (:CastFailed
      _))
  (return true))